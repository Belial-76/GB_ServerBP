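; Multiplayer game mode that splits joining players into two balanced teams.
; On post-login it casts the controller to BP_MultiplayerPlayerController, assigns it to whichever team array is smaller (team 1 on ties), and sets its team ID.
; On logout it removes the controller from the array matching its team ID, re-setting that same ID.
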(event EventPostLogin
  (params (NewPlayer :type Player%20Controller%20Object%20Reference))
  (bind _asbp_multiplayer_player_controller (Utilities|Casting|CastToBP_MultiplayerPlayerController NewPlayer)
    (:then
      (if (< (Utilities|Array|Length (Variables|Default|GetTeam_2)) (Utilities|Array|Length (Variables|Default|GetTeam_1)))
        (Default|SetTeamID _asbp_multiplayer_player_controller 2)
        (Utilities|Array|Add (Variables|Default|GetTeam_2) _asbp_multiplayer_player_controller)
        (else
          (Default|SetTeamID _asbp_multiplayer_player_controller 1)
          (Utilities|Array|Add (Variables|Default|GetTeam_1) _asbp_multiplayer_player_controller))))
    (:CastFailed
      (Development|PrintString "Post login error"))))

(event EventOnLogout
  (params (ExitingController :type Controller%20Object%20Reference))
  (bind _asbp_multiplayer_player_controller (Utilities|Casting|CastToBP_MultiplayerPlayerController ExitingController))
  (if (== (Variables|/Game/Server/BP_MultiplayerPlayerController.BP_MultiplayerPlayerController_C|GetTeamID _asbp_multiplayer_player_controller) 2)
    (Default|SetTeamID _asbp_multiplayer_player_controller 2)
    (Utilities|Array|RemoveItem (Variables|Default|GetTeam_2) _asbp_multiplayer_player_controller)
    (else
      (Default|SetTeamID _asbp_multiplayer_player_controller 1)
      (Utilities|Array|RemoveItem (Variables|Default|GetTeam_1) _asbp_multiplayer_player_controller))))

(fn ConstructionScript)