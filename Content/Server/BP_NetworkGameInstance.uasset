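; Game instance that handles LAN multiplayer sessions: creating, finding and joining games.
; CreateGame uses Advanced Sessions, storing the server name as an extra-setting key with an empty value, then opens Level_1 as a listen server.
; GetGames rebuilds the passed widget's session list with W_Session rows showing name, players and ping.
; JoinToGame joins a chosen result; failures and network or travel errors are only printed.
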(event Custom|CreateGame
  (params (ServerName :type String))
  (|AdvancedSession (Utilities|Array|MakeArray (Class|AdvancedSessionsLibrary|MakeLiteralSessionPropertyString (Utilities|String|StringToName ServerName))) (Game|GetPlayerController 0) 16 0 true true false true true true false false false true
    (:OnSuccess
      (Game|OpenLevel(byName) "Level_1" true "listen"))
    (:OnFailure
      (Development|PrintString "Game creation ERROR!" true true "(R=1.000000,G=0.000000,B=0.006241,A=1.000000)"))))

(event Custom|GetGames
  (params (FindSession :type W%20Find%20Session%20Object%20Reference))
  (bind _sessions (Variables|/Game/Server/W_FindSession.W_FindSession_C|GetSessions FindSession))
  (bind _results (|FindSessions (Game|GetPlayerController 0) 20 true)
    (:OnSuccess
      (Widget|Panel|ClearChildren _sessions)
      (for _array_element _results
        (bind _returnvalue (UserInterface|CreateWidget "/Game/Server/W_Session.W_Session_C"))
        (bind _extrasettings (Class|AdvancedSessionsLibrary|GetExtraSettings _array_element))
        (bind _returnvalue_2 (Class|AdvancedSessionsLibrary|GetSessionPropertyKey (Utilities|Array|Get(acopy) _extrasettings)))
        (Variables|/Game/Server/W_Session.W_Session_C|SetSession _returnvalue _array_element)
        (Rendering|Components|TextRender|SetText (Variables|/Game/Server/W_Session.W_Session_C|GetServerName _returnvalue) (Utilities|Text|ToText(String) (Utilities|String|ToString(Name) _returnvalue_2)))
        (Rendering|Components|TextRender|SetText (Variables|/Game/Server/W_Session.W_Session_C|GetPlaers _returnvalue) (Utilities|Text|ToText(Integer) (Class|FindSessionsCallbackProxy|GetCurrentPlayers _array_element)))
        (Rendering|Components|TextRender|SetText (Variables|/Game/Server/W_Session.W_Session_C|GetPlayersMax _returnvalue) (Utilities|Text|ToText(Integer) (Class|FindSessionsCallbackProxy|GetMaxPlayers _array_element)))
        (Rendering|Components|TextRender|SetText (Variables|/Game/Server/W_Session.W_Session_C|GetPing _returnvalue) (Utilities|Text|ToText(Integer) (Class|FindSessionsCallbackProxy|GetPinginMs _array_element)))
        (Widget|Panel|AddChild _sessions _returnvalue)))
    (:OnFailure
      (Development|PrintString "Game Searching ERROR" true true "(R=1.000000,G=0.000000,B=0.032916,A=1.000000)"))))

(event Custom|JoinToGame
  (params (Session :type Blueprint%20Session%20Result%20Structure))
  (|JoinSession (Game|GetPlayerController 0) Session
    (:OnFailure
      (Development|PrintString "Join to game ERROR" true true "(R=1.000000,G=0.000000,B=0.702509,A=1.000000)"))))

(event EventHandleNetworkError
  (params (FailureType :type ENetworkFailure%20Enum :default "NetDriverAlreadyExists") (bIsServer :type Boolean))
  (Development|PrintString (Utilities|String|Append "Network error: " (Utilities|String|EnumtoString FailureType) " on server?" (Utilities|String|ToString(Boolean) bIsServer))))

(event EventHandleTravelError
  (params (FailureType :type ETravelFailure%20Enum :default "NoLevel"))
  (Development|PrintString (Utilities|String|Append "Network travel error: " (Utilities|String|EnumtoString FailureType))))